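; TheHeckingSun is a visible sun object that matches an assigned directional light.
; The construction script hides the SUN component, then calls SunUpdate, which shows it only if the light is valid.
; SunUpdate places SUN far from the world origin, opposite the light's forward vector, and drives a dynamic material's emissive strength and color from the light's intensity and color.
; The event graph has no runtime logic.
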(event `self.ReceiveBeginPlay`)

(fn `SunUpdate`
  (params (Sun_DirectionalLight :type "DirectionalLight Object Reference"))
  (bind _lightcomponent (`Light.LightComponent` Sun_DirectionalLight))
  (`/Engine/EditorBlueprintResources/StandardMacros.IsValid` Sun_DirectionalLight
    (:`Is Valid`
      (`SceneComponent.SetVisibility` (`self.SUN`) true false)
      (`|ExecutionSequence`
        (:`then_0`
          (`SceneComponent.K2_SetWorldLocation` (`self.SUN`) (* (`SceneComponent.GetForwardVector` (`Actor.RootComponent` Sun_DirectionalLight)) -500000.0) false false))
        (:`then_1`
          (bind _returnvalue (`PrimitiveComponent.CreateDynamicMaterialInstance` (`self.SUN`) 0 "/Game/CrazedObjectsHouse/Materials/mat_basic.mat_basic"))
          (bind _output_get (set `self.SunMaterialDynamic` _returnvalue))
          (`MaterialInstanceDynamic.SetScalarParameterValue` _returnvalue "EmissiveStrength" (`LightComponentBase.Intensity` _lightcomponent))
          (`MaterialInstanceDynamic.SetScalarParameterValue` _output_get "EmissiveStrength" (`LightComponentBase.Intensity` _lightcomponent))
          (`MaterialInstanceDynamic.SetVectorParameterValue` (`self.SunMaterialDynamic`) "Color" (`LightComponentBase.GetLightColor` _lightcomponent)))))))

(fn `UserConstructionScript`
  (bind _sun (`self.SUN`))
  (`SceneComponent.SetVisibility` _sun false false)
  (bind _returnvalue (`PrimitiveComponent.CreateDynamicMaterialInstance` _sun 0 "/Game/CrazedObjectsHouse/Materials/mat_basic.mat_basic"))
  (set `self.SunMaterialDynamic` _returnvalue)
  (`self.SunUpdate` (`self.ActiveDirLight`)))
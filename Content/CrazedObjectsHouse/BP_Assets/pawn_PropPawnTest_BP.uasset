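; Test pawn for a prop, set up to wander by AI move to random navigable points within a walk radius.
; Tick holds the move logic, which sets a Walking flag on start and clears it on success or failure.
; That logic sits on the false side of a constant-true branch, so it never executes.
; A delayed, random-direction debug line trace from the static mesh is also left unconnected.
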(event `self.ReceiveTick`
  (params (DeltaSeconds :type "Float (single-precision)"))
  (if (not true)
    (`|AIMoveTo` self (`NavigationSystem.K2_GetRandomLocationInNavigableRadius` (`self.K2_GetActorLocation`) (`self.WalkRadius`))
      (:`then`
        (set `self.Walking?` true))
      (:`OnSuccess`
        (set `self.Walking?` false :!label _label))
      (:`OnFail`
        (goto _label)))))

(fn `UserConstructionScript`)
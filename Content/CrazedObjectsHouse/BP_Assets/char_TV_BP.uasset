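; AI character for a TV that wanders to random navigable points at a randomized speed, chasing the player when they hold the remote.
; Pawn sensing stores the player, and a looping WalkEvent picks wander or follow, tinting the prop white or green.
; PutAsleep darkens it and enables capsule physics for a timed sleep, extended while the overlapped player's PickUp is set.
; Waking, also triggered by player overlap, disables physics and resumes walking.
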(event `WalkEvent`
  (if (`self.IsAsleep`)
    ;[1 1 1] Walk Logic
    (`KismetSystemLibrary.Delay` (`self.SleepTime`))
    (else
      (if (`/Game/CrazedObjectsHouse/BP_Assets/char_FirstPersonCharacter.PLAYERREMOTE` (stale `self.PawnSensing.OnSeePawn` _aschar_first_person_character)) :!label _label
        (bind _returnvalue (`PrimitiveComponent.CreateDynamicMaterialInstance` (`self.Prop`) 0 "/Game/CrazedObjectsHouse/Materials/Debug/mat_CorrectSpotTrigger_mat.mat_CorrectSpotTrigger_mat"))
        (`MaterialInstanceDynamic.SetVectorParameterValue` _returnvalue "Color" (struct :`R` 0.116857 :`G` 0.848958 :`B` 0.039795 :`A` 1.0))
        (`|AIMoveTo` self (`SceneComponent.K2_GetComponentLocation` (`Actor.RootComponent` (stale `self.PawnSensing.OnSeePawn` _aschar_first_person_character)))
          (:`OnSuccess`
            (goto _label)))
        (else
          (bind _returnvalue_2 (`PrimitiveComponent.CreateDynamicMaterialInstance` (`self.Prop`) 0 "/Game/CrazedObjectsHouse/Materials/Debug/mat_CorrectSpotTrigger_mat.mat_CorrectSpotTrigger_mat"))
          (`MaterialInstanceDynamic.SetVectorParameterValue` _returnvalue_2 "Color" (struct :`R` 1.0 :`G` 1.0 :`B` 1.0 :`A` 1.0))
          (`KismetSystemLibrary.PrintString` "Im awake" true true (struct :`R` 0.401042 :`G` 0.040587 :`B` 0.23413 :`A` 1.0))))))
  (if (not (`self.Walking`))
    (`|AIMoveTo` self (`NavigationSystem.K2_GetRandomLocationInNavigableRadius` (`self.K2_GetActorLocation`) (`self.WalkRadius`))
      (:`then`
        (set `self.Walking` true))
      (:`OnSuccess`
        (`KismetSystemLibrary.Delay` (`KismetMathLibrary.RandomFloatInRange` 1.0 2.0) :!label _label_2)
        (set `self.Walking` false)
        (`self.WalkEvent`))
      (:`OnFail`
        (goto _label_2)))))

(event `self.ReceiveBeginPlay`
  (`PrimitiveComponent.SetSimulatePhysics` (`self.CapsuleComponent`) true)
  (`KismetSystemLibrary.Delay` 0.2)
  (`PrimitiveComponent.SetSimulatePhysics` (`self.CapsuleComponent`) false)
  ;[1 1 1] Walk Logic
  (bind _output_get (set `self.WalkSpeed` (`KismetMathLibrary.RandomFloatInRange` 200.0 600.0)))
  (set `CharacterMovementComponent.MaxWalkSpeed` _output_get (`self.CharacterMovement`))
  (`self.WalkEvent`)
  (set `self.IsAsleep` false))

(event `self.PawnSensing.OnSeePawn`
  (params (Pawn :type "Pawn Object Reference"))
  (bind _aschar_first_person_character (cast `/Game/CrazedObjectsHouse/BP_Assets/char_FirstPersonCharacter` Pawn)))

(event `PutAsleep`
  (set `self.IsAsleep` true)
  (`PrimitiveComponent.SetSimulatePhysics` (`self.CapsuleComponent`) true)
  (`KismetSystemLibrary.PrintString` "Im asleep" :!label _label_3)
  (bind _returnvalue (`PrimitiveComponent.CreateDynamicMaterialInstance` (`self.Prop`) 0 "/Game/CrazedObjectsHouse/Materials/Debug/mat_CorrectSpotTrigger_mat.mat_CorrectSpotTrigger_mat"))
  (`MaterialInstanceDynamic.SetVectorParameterValue` _returnvalue "Color" (struct :`R` 0.014993 :`G` 0.012086 :`B` 0.03125 :`A` 1.0))
  (`KismetSystemLibrary.Delay` (`self.SleepTime`))
  (if (`/Game/CrazedObjectsHouse/BP_Assets/char_FirstPersonCharacter.PickUp` (stale `self.ReceiveActorBeginOverlap` _aschar_first_person_character)) :!label _label_4
    (goto _label_3)
    (else
      (set `self.IsAsleep` false)
      (`PrimitiveComponent.SetSimulatePhysics` (`self.CapsuleComponent`) false)
      (`self.K2_SetActorLocationAndRotation` (`SceneComponent.K2_GetComponentLocation` (`self.CapsuleComponent`)))
      (`self.WalkEvent`)
      (`KismetSystemLibrary.PrintString` "Im awake" true true (struct :`R` 0.401042 :`G` 0.040587 :`B` 0.23413 :`A` 1.0))
      (bind _returnvalue_2 (`PrimitiveComponent.CreateDynamicMaterialInstance` (`self.Prop`) 0 "/Game/CrazedObjectsHouse/Materials/Debug/mat_CorrectSpotTrigger_mat.mat_CorrectSpotTrigger_mat"))
      (`MaterialInstanceDynamic.SetVectorParameterValue` _returnvalue_2 "Color" (struct :`R` 1.0 :`G` 1.0 :`B` 1.0 :`A` 1.0)))))

(event `self.ReceiveActorBeginOverlap`
  (params (OtherActor :type "Actor Object Reference"))
  (bind _aschar_first_person_character (cast `/Game/CrazedObjectsHouse/BP_Assets/char_FirstPersonCharacter` OtherActor))
  (goto _label_4))

(event `Player Has remote`)

(fn `UserConstructionScript`)
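; Test prop character that wanders the navmesh and can be put to sleep, apparently so the player can carry it.
; WalkEvent loops AIMoveTo to random nearby points at a randomized speed, pausing briefly between moves.
; PutAsleep enables capsule physics and darkens the prop's dynamic material, rechecking after SleepTime and staying asleep while the player's PickUp is set.
; Player overlap caches that character and jumps straight into the same sleep-or-wake check.
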(event `self.ReceiveTick`
  (params (DeltaSeconds :type "Float (single-precision)")))

(event `self.ReceiveBeginPlay`
  ;[1 1 1] Walk Logic
  (`PrimitiveComponent.SetSimulatePhysics` (`self.CapsuleComponent`) true)
  (`KismetSystemLibrary.Delay` 0.2)
  (`PrimitiveComponent.SetSimulatePhysics` (`self.CapsuleComponent`) false)
  (bind _output_get (set `self.WalkSpeed` (`KismetMathLibrary.RandomFloatInRange` 100.0 450.0)))
  (set `CharacterMovementComponent.MaxWalkSpeed` _output_get (`self.CharacterMovement`))
  (`self.WalkEvent`)
  (set `self.IsAsleep` false))

(event `WalkEvent`
  ;[1 1 1] Walk Logic
  (bind _returnvalue (`PrimitiveComponent.CreateDynamicMaterialInstance` (`self.Prop`) 0 "/Game/CrazedObjectsHouse/Materials/Debug/mat_CorrectSpotTrigger_mat.mat_CorrectSpotTrigger_mat"))
  (`MaterialInstanceDynamic.SetVectorParameterValue` _returnvalue "Color" (struct :`R` 1.0 :`G` 1.0 :`B` 1.0 :`A` 1.0))
  (if (`self.IsAsleep`)
    (`KismetSystemLibrary.Delay` (`self.SleepTime`))
    (else
      (`KismetSystemLibrary.PrintString` "Im awake" true true (struct :`R` 0.401042 :`G` 0.040587 :`B` 0.23413 :`A` 1.0))))
  (if (not (`self.Walking`))
    (`|AIMoveTo` self (`NavigationSystem.K2_GetRandomLocationInNavigableRadius` (`self.K2_GetActorLocation`) (`self.WalkRadius`))
      (:`then`
        (set `self.Walking` true))
      (:`OnSuccess`
        (`KismetSystemLibrary.Delay` (`KismetMathLibrary.RandomFloatInRange` 1.0 3.0) :!label _label)
        (set `self.Walking` false)
        (`self.WalkEvent`))
      (:`OnFail`
        (goto _label)))))

(event `PutAsleep`
  (set `self.IsAsleep` true)
  (`PrimitiveComponent.SetSimulatePhysics` (`self.CapsuleComponent`) true)
  (`KismetSystemLibrary.PrintString` "Im asleep" :!label _label_2)
  (bind _returnvalue (`PrimitiveComponent.CreateDynamicMaterialInstance` (`self.Prop`) 0 "/Game/CrazedObjectsHouse/Materials/Debug/mat_CorrectSpotTrigger_mat.mat_CorrectSpotTrigger_mat"))
  (`MaterialInstanceDynamic.SetVectorParameterValue` _returnvalue "Color" (struct :`R` 0.014993 :`G` 0.012086 :`B` 0.03125 :`A` 1.0))
  (`KismetSystemLibrary.Delay` (`self.SleepTime`))
  (if (`/Game/CrazedObjectsHouse/BP_Assets/char_FirstPersonCharacter.PickUp` (stale `self.ReceiveActorBeginOverlap` _aschar_first_person_character)) :!label _label_3
    (goto _label_2)
    (else
      (set `self.IsAsleep` false)
      (`PrimitiveComponent.SetSimulatePhysics` (`self.CapsuleComponent`) false)
      (`self.K2_SetActorLocationAndRotation` (`SceneComponent.K2_GetComponentLocation` (`self.CapsuleComponent`)))
      (`self.WalkEvent`)
      (`KismetSystemLibrary.PrintString` "Im awake" true true (struct :`R` 0.401042 :`G` 0.040587 :`B` 0.23413 :`A` 1.0))
      (bind _returnvalue_2 (`PrimitiveComponent.CreateDynamicMaterialInstance` (`self.Prop`) 0 "/Game/CrazedObjectsHouse/Materials/Debug/mat_CorrectSpotTrigger_mat.mat_CorrectSpotTrigger_mat"))
      (`MaterialInstanceDynamic.SetVectorParameterValue` _returnvalue_2 "Color" (struct :`R` 1.0 :`G` 1.0 :`B` 1.0 :`A` 1.0)))))

(event `self.ReceiveActorBeginOverlap`
  (params (OtherActor :type "Actor Object Reference"))
  (bind _aschar_first_person_character (cast `/Game/CrazedObjectsHouse/BP_Assets/char_FirstPersonCharacter` OtherActor))
  (goto _label_3))

(fn `UserConstructionScript`)